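; BP_BaseAI is a base enemy AI that detects pawns, fires projectiles and reports to the game manager when destroyed.
; Pawn sensing stores the seen pawn as its target, while capsule hits snap its rotation to face the player.
; ShootProjectile spawns a BP_BaseProjectile from the mesh's FireSocket, and DestroyAI passes a count change and XP reward to GameManager before destroying the actor.
; BeginPlay registers it as owner of its HealthComponent.
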(event OnComponentHit(CapsuleComponent)
  (params (HitComponent :type Primitive%20Component%20Object%20Reference) (OtherActor :type Actor%20Object%20Reference) (OtherComp :type Primitive%20Component%20Object%20Reference) (NormalImpulse :type Vector) (Hit :type Hit%20Result%20Structure%20%28by%20ref%29))
  (Transformation|SetActorRotation (Math|Rotator|FindLookatRotation (Transformation|GetActorLocation) (Transformation|GetActorLocation (Game|GetPlayerCharacter 0)))))

(event OnSeePawn(PawnSensing)
  (params (Pawn :type Pawn%20Object%20Reference))
  (Variables|Default|SetDetectedTarget Pawn)
  (Variables|Default|SetHasTarget true))

(event EventBeginPlay
  (Variables|/Game/Blueprints/BP_HealthComponent.BP_HealthComponent_C|SetOwner (Variables|Default|GetHealthComponent) self))

(event Collision|EventActorBeginOverlap
  (params (OtherActor :type Actor%20Object%20Reference)))

(event EventTick
  (params (DeltaSeconds :type Float%20%28single-precision%29)))

(fn ConstructionScript)

(fn ShootProjectile
  (Game|SpawnActorfromClass "/Game/Blueprints/BP_BaseProjectile.BP_BaseProjectile_C" (Transformation|GetSocketTransform (Variables|Default|GetStaticMesh) "FireSocket" "RTS_World") "Undefined" 0 5e+02 5e+02 1.0 1e+01))

(fn DestroyAI
  (Default|ChangeAICount (Variables|Default|GetGameManager) 1 (Variables|Default|GetXPReward))
  (Actor|DestroyActor))