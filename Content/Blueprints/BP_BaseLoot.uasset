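; BP_BaseLoot is a base loot pickup actor that applies its reward to the main character on hit.
; GetDataFromDB fills LootType and Value from a named row in the DB_DropList data table, but is not called within this Blueprint.
; On Hit, PassData casts the other actor to BP_MainCharacter and handles only XP Boost, via the PlayerController's UpdateXP.
; The actor then destroys itself, whatever it hit.
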(event EventBeginPlay)

(event Collision|EventActorBeginOverlap
  (params (OtherActor :type Actor%20Object%20Reference)))

(event Collision|EventHit
  (params (MyComp :type Primitive%20Component%20Object%20Reference) (Other :type Actor%20Object%20Reference) (OtherComp :type Primitive%20Component%20Object%20Reference) (bSelfMoved :type Boolean) (HitLocation :type Vector :default "0, 0, 0") (HitNormal :type Vector :default "0, 0, 0") (NormalImpulse :type Vector :default "0, 0, 0") (Hit :type Hit%20Result%20Structure%20%28by%20ref%29))
  (CallFunction|PassData Other)
  (Actor|DestroyActor))

(event EventTick
  (params (DeltaSeconds :type Float%20%28single-precision%29)))

(fn ConstructionScript)

(fn PassData
  (params (Actor :type Actor%20Object%20Reference))
  (bind _asbp_main_character (Utilities|Casting|CastToBP_MainCharacter Actor))
  (Variables|Default|SetMainCharacter _asbp_main_character)
  (switch Utilities|FlowControl|Switch|SwitchonEN_LootType (Variables|Default|GetLootType)
    (:NewEnumerator2
      (Default|UpdateXP (Variables|/Game/Blueprints/Core/BP_MainCharacter.BP_MainCharacter_C|GetPlayerController (Variables|Default|GetMainCharacter)) (Math|Float|Truncate (Variables|Default|GetValue))))))

(fn GetDatafromDB
  (params (ObjectName :type Name))
  (bind _returnvalue (Utilities|GetDataTableRow "/Game/Blueprints/DB_DropList.DB_DropList" ObjectName)
    (:then
      (Utilities|FlowControl|Sequence
        (:then_0
          (Variables|Default|SetLootType (.LootType (Utilities|Struct|BreakS_DropItem _returnvalue))))
        (:then_1
          (Variables|Default|SetValue (.Value (Utilities|Struct|BreakS_DropItem _returnvalue))))))))