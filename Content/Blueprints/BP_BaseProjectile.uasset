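; BP_BaseProjectile is a projectile actor that damages BP_BaseAI actors it hits.
; Its construction script copies InitialSpeed and MaxSpeed into ProjectileMovement, and BeginPlay destroys it after Lifetime.
; On Hit, a damageable actor of exactly the BP_BaseAI class, not a child class, receives ProjectileDamage through its HealthComponent, and the projectile destroys itself.
; Other hits leave it alive until the lifetime expires.
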(event EventBeginPlay
  (Utilities|FlowControl|Delay (Variables|Default|GetLifetime))
  (Actor|DestroyActor))

(event Collision|EventActorBeginOverlap
  (params (OtherActor :type Actor%20Object%20Reference)))

(event Collision|EventHit
  (params (MyComp :type Primitive%20Component%20Object%20Reference) (Other :type Actor%20Object%20Reference) (OtherComp :type Primitive%20Component%20Object%20Reference) (bSelfMoved :type Boolean) (HitLocation :type Vector :default "0, 0, 0") (HitNormal :type Vector :default "0, 0, 0") (NormalImpulse :type Vector :default "0, 0, 0") (Hit :type Hit%20Result%20Structure%20%28by%20ref%29))
  (if (Variables|/Script/Engine.Actor|GetbCanBeDamaged Other)
    (if (== (Utilities|GetClass Other) "/Game/Blueprints/AI/BP_BaseAI.BP_BaseAI_C")
      (bind _asbp_base_ai (Utilities|Casting|CastToBP_BaseAI Other))
      (Default|GetDamage (Variables|/Game/Blueprints/AI/BP_BaseAI.BP_BaseAI_C|GetHealthComponent _asbp_base_ai) (Variables|Default|GetProjectileDamage))
      (Actor|DestroyActor))))

(event EventTick
  (params (DeltaSeconds :type Float%20%28single-precision%29)))

(fn ConstructionScript
  (bind _projectilemovement (Variables|Default|GetProjectileMovement))
  (Variables|/Script/Engine.ProjectileMovementComponent|SetInitialSpeed _projectilemovement (Variables|Default|GetInitialSpeed))
  (Variables|/Script/Engine.ProjectileMovementComponent|SetMaxSpeed _projectilemovement (Variables|Default|GetMaxSpeed)))