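; Health component that tracks its owning actor's health, regenerates it and destroys the actor when health drops below zero.
; On BeginPlay, SetHealthCap derives the cap from base plus bonus health, and GetDamage subtracts incoming damage from current health.
; Each Tick checks for death, then adds base and bonus regen while health is at or below the cap, without delta-time scaling or clamping.
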(event EventBeginPlay
  (CallFunction|SetHealthCap (Variables|Default|GetBonusHealth)))

(event EventTick
  (params (DeltaSeconds :type Float%20%28single-precision%29))
  (Utilities|FlowControl|Sequence
    (:then_0
      (if (< (Variables|Default|GetCurrentHealth) 0.0)
        (Actor|DestroyActor (Variables|Default|GetOwner))))
    (:then_1
      (if (<= (Variables|Default|GetCurrentHealth) (Variables|Default|GetHealthCap))
        (Variables|Default|SetCurrentHealth (+ (Variables|Default|GetCurrentHealth) (Variables|Default|GetBaseHealthRegen) (Variables|Default|GetBonusHealthRegen)))))))

(fn SetHealthCap
  (params (Bonus :type Float%20%28single-precision%29))
  (Variables|Default|SetHealthCap (+ Bonus (Variables|Default|GetBaseHealth))))

(fn GetDamage
  (params (Damage :type Float%20%28single-precision%29))
  (Variables|Default|SetCurrentHealth (- (Variables|Default|GetCurrentHealth) Damage)))