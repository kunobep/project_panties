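; BP_BaseSpawn is a spawner actor that creates AI pawns at its own location when play begins.
; It loops over the SpawnEntity class list, spawns each with the BT_BaseAI behavior tree and passes its GameManager reference to the resulting BP_BaseAI.
; An unconnected node that would set the manager's KillLimit from the list length never runs.
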(event EventBeginPlay
  (for _array_element (Variables|Default|GetSpawnEntity)
    (bind _returnvalue (AI|SpawnAIFromClass _array_element "/Game/Blueprints/AI/BT_BaseAI.BT_BaseAI" (.Location (Math|Transform|BreakTransform (Transformation|GetActorTransform))) "0, 0, 0" false))
    (bind _asbp_base_ai (Utilities|Casting|CastToBP_BaseAI _returnvalue))
    (Variables|/Game/Blueprints/AI/BP_BaseAI.BP_BaseAI_C|SetGameManager _asbp_base_ai (Variables|Default|GetGameManager))))

(event Collision|EventActorBeginOverlap
  (params (OtherActor :type Actor%20Object%20Reference)))

(event EventTick
  (params (DeltaSeconds :type Float%20%28single-precision%29)))

(fn ConstructionScript)