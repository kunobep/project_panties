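; First-person player character Blueprint that handles movement, mouse look, weapon firing and the death screen.
; Left-action input checks the current weapon's ammo, then spawns a projectile at the gun's ShootTransform socket using that weapon's stats, without decrementing ammo here.
; Damage is forwarded to HealthComponent, whose health is copied to PlayerHealth every tick.
; SetDead shows the end-of-round defeat screen with zeroed kill and XP values.
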(event EventBeginPlay
  (Variables|/Game/Blueprints/BP_HealthComponent.BP_HealthComponent_C|SetOwner (Variables|Default|GetHealthComponent) self)
  (bind _asbp_fpscontroller (Utilities|Casting|CastToBP_FPSController (Game|GetPlayerController 0)))
  (Variables|Default|SetPlayerController _asbp_fpscontroller))

(event Collision|EventActorBeginOverlap
  (params (OtherActor :type Actor%20Object%20Reference)))

(event EventTick
  (params (DeltaSeconds :type Float%20%28single-precision%29))
  (Variables|Default|SetPlayerHealth (Variables|/Game/Blueprints/BP_HealthComponent.BP_HealthComponent_C|GetCurrentHealth (Variables|Default|GetHealthComponent))))

(event Input|ActionEvents|InputActionLeftAction
  (params (Key :type Key%20Structure :default "AnyKey"))
  (:Pressed
    (if (> (Variables|/Game/Blueprints/BP_Weapon.BP_Weapon_C|GetRemaingAmmo (Variables|Default|GetWeapon)) 0.0)
      (bind (_projectilevelocity _projectiledamage _projectilelifetime) (Default|GetProjectileStats (Variables|Default|GetWeapon)))
      (bind _returnvalue (Game|SpawnActorfromClass "/Game/Blueprints/BP_BaseProjectile.BP_BaseProjectile_C" (Transformation|GetSocketTransform (Variables|Default|GetBaseGun) "ShootTransform" "RTS_World") "AdjustIfPossibleButDontSpawnIfColliding" 0 _projectilevelocity _projectilevelocity _projectiledamage _projectilelifetime))
      (Actor|SetLifeSpan _returnvalue 1.0))))

(event Input|AxisEvents|InputAxisMoveForward
  (params (AxisValue :type Float%20%28single-precision%29))
  (Pawn|Input|AddMovementInput (Transformation|GetActorForwardVector) AxisValue false))

(event Input|AxisEvents|InputAxisMoveRight
  (params (AxisValue :type Float%20%28single-precision%29))
  (Pawn|Input|AddMovementInput (Transformation|GetActorRightVector) AxisValue false))

(event Input|AxisEvents|InputAxisTurn
  (params (AxisValue :type Float%20%28single-precision%29))
  (Pawn|Input|AddControllerYawInput AxisValue))

(event Input|AxisEvents|InputAxisLookUp
  (params (AxisValue :type Float%20%28single-precision%29))
  (Pawn|Input|AddControllerPitchInput AxisValue))

(fn ConstructionScript)

(fn ReturnCurrentWeapon
  (return (Variables|Default|GetWeapon)))

(fn LoadWeapon
  (params (Weapon :type BP%20Weapon%20Object%20Reference))
  (Variables|Default|SetWeapon Weapon))

(fn SetDead
  (Default|ShowEORScreen (Variables|Default|GetMainHUD) 0 0 false))

(fn GetDamage
  (params (Damage :type Float%20%28single-precision%29))
  (Default|GetDamage (Variables|Default|GetHealthComponent) Damage))