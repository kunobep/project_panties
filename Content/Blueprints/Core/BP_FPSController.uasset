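; Player controller for an FPS that links the main character and HUD, spawns the weapon, and tracks free XP.
; On BeginPlay it reads GameState from the game manager, then spawns the weapon and loads saved components and XP in menu or game.
; Loading ignores its slot argument, chaining from "SaveGameSlot" to the stored slot name.
; Debug inputs save with an empty slot name or damage the player.
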(event Custom|GetCoreBP
  (Utilities|FlowControl|Sequence
    (:then_0
      (bind _asbp_main_character (Utilities|Casting|CastToBP_MainCharacter (Game|GetPlayerCharacter 0)))
      (bind _output_get (Variables|Default|SetPlayerCharacter _asbp_main_character))
      (Variables|/Game/Blueprints/Core/BP_MainCharacter.BP_MainCharacter_C|SetMainHUD _output_get (stale _output_get_2)))
    (:then_1
      (bind _asbp_main_hud (Utilities|Casting|CastToBP_MainHUD (HUD|GetHUD)))
      (bind _output_get_2 (Variables|Default|SetMainHUD _asbp_main_hud))
      (Variables|/Game/Blueprints/Core/BP_MainHUD.BP_MainHUD_C|SetPlayerCharacter _output_get_2 _output_get))
    (:then_2
      (CallFunction|UpdateGameState))))

(event EventBeginPlay
  (CallFunction|GetCoreBP)
  (switch Utilities|FlowControl|Switch|SwitchonEN_GameModeState (Variables|Default|GetGameState)
    (:NewEnumerator1
      _)
    (:NewEnumerator2
      _))
  (CallFunction|LoadWeapon)
  (CallFunction|LoadGameData))

(event EventTick
  (params (DeltaSeconds :type Float%20%28single-precision%29)))

(event Input|ActionEvents|InputActionHelp1
  (params (Key :type Key%20Structure :default "AnyKey"))
  (:Pressed
    (CallFunction|SaveGameData)))

(event Input|ActionEvents|InputActionHelp2
  (params (Key :type Key%20Structure :default "AnyKey"))
  (:Pressed
    (Default|GetDamage (Variables|Default|GetPlayerCharacter) 1.0)))

(fn ConstructionScript)

(fn LoadGameData
  (params (SlotName :type String))
  (SaveGame|CreateSaveGameObject "/Game/Blueprints/Core/BP_SaveGame.BP_SaveGame_C")
  (bind _returnvalue (SaveGame|LoadGamefromSlot "SaveGameSlot"))
  (bind _asbp_save_game (Utilities|Casting|CastToBP_SaveGame _returnvalue))
  (bind _returnvalue_2 (SaveGame|LoadGamefromSlot (Variables|/Game/Blueprints/Core/BP_SaveGame.BP_SaveGame_C|GetSaveSlot _asbp_save_game)))
  (bind _asbp_save_game_2 (Utilities|Casting|CastToBP_SaveGame _returnvalue_2))
  (Variables|Default|SetSaveGame _asbp_save_game_2)
  (Utilities|FlowControl|Sequence
    (:then_0
      (Variables|/Game/Blueprints/BP_Weapon.BP_Weapon_C|SetWeaponComponentList (Variables|Default|GetWeapon) (Variables|/Game/Blueprints/Core/BP_SaveGame.BP_SaveGame_C|GetWeaponComponents (Variables|Default|GetSaveGame))))
    (:then_1
      (Variables|Default|SetMainCharacterFreeXP (Variables|/Game/Blueprints/Core/BP_SaveGame.BP_SaveGame_C|GetMainCharacterFreeXP (Variables|Default|GetSaveGame))))))

(fn SaveGameData
  (params (SlotName :type String))
  (bind _returnvalue (SaveGame|CreateSaveGameObject "/Game/Blueprints/Core/BP_SaveGame.BP_SaveGame_C"))
  (bind _asbp_save_game (Utilities|Casting|CastToBP_SaveGame _returnvalue))
  (Variables|Default|SetSaveGame _asbp_save_game)
  (Variables|/Game/Blueprints/Core/BP_SaveGame.BP_SaveGame_C|SetWeaponComponents (Variables|Default|GetSaveGame) (Variables|/Game/Blueprints/BP_Weapon.BP_Weapon_C|GetWeaponComponentList (Variables|Default|GetWeapon)))
  (Variables|/Game/Blueprints/Core/BP_SaveGame.BP_SaveGame_C|SetMainCharacterFreeXP (Variables|Default|GetSaveGame) (Variables|Default|GetMainCharacterFreeXP))
  (SaveGame|SaveGametoSlot (Variables|Default|GetSaveGame) SlotName))

(fn LoadWeapon
  (bind _returnvalue (Game|SpawnActorfromClass "/Game/Blueprints/BP_Weapon.BP_Weapon_C" (Math|Transform|MakeTransform "0, 0, 0") "Undefined" 0 0))
  (Variables|Default|SetWeapon _returnvalue)
  (Default|LoadWeapon (Variables|Default|GetPlayerCharacter) (Variables|Default|GetWeapon))
  (Default|LinkHUD (Variables|Default|GetWeapon) (Variables|Default|GetMainHUD)))

(fn UpdateGameState
  (bind _outactors (Actor|GetAllActorsOfClass "/Game/Blueprints/Core/BP_GameManager.BP_GameManager_C"))
  (Variables|Default|SetGameState (Variables|/Game/Blueprints/Core/BP_GameManager.BP_GameManager_C|GetGameState (Utilities|Array|Get(acopy) _outactors))))

(fn UpdateXP
  (params (XPCount :type Integer))
  (bind _output_get (Variables|Default|SetMainCharacterFreeXP (+ XPCount (Variables|Default|GetMainCharacterFreeXP))))
  (Default|UpdateXP (Variables|Default|GetMainHUD) _output_get))