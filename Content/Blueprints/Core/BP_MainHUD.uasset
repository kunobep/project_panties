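; HUD class that shows the main menu, world menu or in-game stats widget according to the FPS controller's GameState.
; On BeginPlay it creates the matching widget and sets UI-only input for menus or game-only input for gameplay.
; During gameplay it pushes player health to UI_MainParams every Tick.
; Free XP is set when that widget loads, and UpdateXP and UpdateEnemy forward later values to it.
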(event EventBeginPlay
  (bind _returnvalue (Game|GetPlayerController 0))
  (bind _asbp_fpscontroller (Utilities|Casting|CastToBP_FPSController (Game|GetPlayerController 0)))
  (bind _output_get (Variables|Default|SetFPSController _asbp_fpscontroller))
  (switch Utilities|FlowControl|Switch|SwitchonEN_GameModeState (Variables|/Game/Blueprints/Core/BP_FPSController.BP_FPSController_C|GetGameState _output_get)
    (:NewEnumerator0
      (CallFunction|LoadMainMenu)
      (Input|SetInputModeUIOnly _returnvalue 0 "DoNotLock" :!label _label))
    (:NewEnumerator1
      (CallFunction|LoadWorldMenu)
      (goto _label))
    (:NewEnumerator2
      (CallFunction|LoadMainWidgets)
      (Input|SetInputModeGameOnly _returnvalue))))

(event Collision|EventActorBeginOverlap
  (params (OtherActor :type Actor%20Object%20Reference)))

(event EventTick
  (params (DeltaSeconds :type Float%20%28single-precision%29))
  (switch Utilities|FlowControl|Switch|SwitchonEN_GameModeState (Variables|/Game/Blueprints/Core/BP_FPSController.BP_FPSController_C|GetGameState (Variables|Default|GetFPSController))
    (:NewEnumerator2
      (CallFunction|UpdateHealth (Variables|/Game/Blueprints/Core/BP_MainCharacter.BP_MainCharacter_C|GetPlayerHealth (Variables|Default|GetPlayerCharacter))))))

(fn ConstructionScript)

(fn LoadMainWidgets
  (Utilities|FlowControl|Sequence
    (:then_0
      (bind _returnvalue (UserInterface|CreateWidget "/Game/Blueprints/UI/UI_MainParams.UI_MainParams_C" (Game|Player|GetOwningPlayerController)))
      (bind _output_get (Variables|Widgets|SetMainParamsWidget _returnvalue))
      (UserInterface|Viewport|AddtoViewport _output_get 0)
      (Utilities|FlowControl|Sequence
        (:then_0
          (CallFunction|UpdateXP (Variables|/Game/Blueprints/Core/BP_FPSController.BP_FPSController_C|GetMainCharacterFreeXP (Variables|Default|GetFPSController))))))))

(fn UpdateHealth
  (params (Health :type Float%20%28single-precision%29))
  (Default|UpdateHealth (Variables|Widgets|GetMainParamsWidget) Health))

(fn LoadMainMenu
  (bind _returnvalue (UserInterface|CreateWidget "/Game/Blueprints/UI/UI_MainMenu.UI_MainMenu_C" (Game|Player|GetOwningPlayerController)))
  (bind _output_get (Variables|Widgets|SetMainMenuWidget _returnvalue))
  (Variables|/Game/Blueprints/UI/UI_MainMenu.UI_MainMenu_C|SetPlayerController _output_get (Variables|Default|GetFPSController))
  (UserInterface|Viewport|AddtoViewport _output_get 0))

(fn LoadWorldMenu
  (bind _returnvalue (UserInterface|CreateWidget "/Game/Blueprints/UI/UI_WorldMenu.UI_WorldMenu_C" (Game|Player|GetOwningPlayerController)))
  (bind _output_get (Variables|Widgets|SetWorldMenuWidget _returnvalue))
  (Variables|/Game/Blueprints/UI/UI_WorldMenu.UI_WorldMenu_C|SetPlayerController _output_get (Variables|Default|GetFPSController))
  (UserInterface|Viewport|AddtoViewport _output_get 0))

(fn UpdateXP
  (params (CurrentFreeXP :type Integer))
  (Default|UpdateXP (Variables|Widgets|GetMainParamsWidget) CurrentFreeXP))

(fn UpdateEnemy
  (params (EnemyCount :type Integer))
  (Default|UpdateEnemy (Variables|Widgets|GetMainParamsWidget) EnemyCount))