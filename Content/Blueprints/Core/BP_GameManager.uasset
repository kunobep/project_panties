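; Game manager that tracks the remaining kill count and triggers victory when it runs out.
; On BeginPlay it caches the FPS player controller, hands it a self-reference, and sends the kill limit to the main HUD.
; ChangeAICount lowers the limit, updates HUD and player XP, and shows the end-of-round victory screen at zero or below, passing zeroed stats.
; LoadSaveData is an empty stub.
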(event EventBeginPlay
  (Utilities|FlowControl|Sequence
    (:then_0
      (bind _asbp_fpscontroller (Utilities|Casting|CastToBP_FPSController (Game|GetPlayerController 0)))
      (bind _output_get (Variables|Default|SetPlayerController _asbp_fpscontroller))
      (Variables|/Game/Blueprints/Core/BP_FPSController.BP_FPSController_C|SetGameManager _output_get self))
    (:then_1
      (bind _asbp_main_hud (Utilities|Casting|CastToBP_MainHUD (HUD|GetHUD (Variables|Default|GetPlayerController))))
      (bind _output_get_2 (Variables|Default|SetMainHUD _asbp_main_hud))
      (Default|UpdateEnemy _output_get_2 (Variables|Default|GetKillLimit)))))

(event Collision|EventActorBeginOverlap
  (params (OtherActor :type Actor%20Object%20Reference)))

(event EventTick
  (params (DeltaSeconds :type Float%20%28single-precision%29)))

(fn ConstructionScript)

(fn ChangeAICount
  (params (AIDifference :type Integer) (XPReward :type Integer))
  (bind _output_get (Variables|Default|SetKillLimit (- (Variables|Default|GetKillLimit) AIDifference)))
  (Default|UpdateEnemy (Variables|Default|GetMainHUD) _output_get)
  (Default|UpdateXP (Variables|Default|GetPlayerController) XPReward)
  (if (<= (Variables|Default|GetKillLimit) 0)
    (Default|ShowEORScreen (Variables|Default|GetMainHUD) 0 0 true)))

(fn LoadSaveData)