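; BP_Weapon is a weapon Blueprint that derives projectile stats from the components attached to it.
; GetProjectileStats loops over each entry in WeaponComponents and its WeaponBonus list, switching on the bonus parameter.
; Projectile Speed bonuses are added onto BulletVelocity, which the function returns.
; The event graph and construction script hold no logic.
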(event EventBeginPlay)

(event Collision|EventActorBeginOverlap
  (params (OtherActor :type Actor%20Object%20Reference)))

(event EventTick
  (params (DeltaSeconds :type Float%20%28single-precision%29)))

(fn ConstructionScript)

(fn GetProjectileStats
  (for _array_element (Variables|Default|GetWeaponComponents)
    (for _array_element_2 (.WeaponBonus (Utilities|Struct|BreakS_WeaponComponent _array_element))
      (switch Utilities|FlowControl|Switch|SwitchonE_WeaponBonusType (.BonusParameter (Utilities|Struct|BreakS_WeaponBonus _array_element_2))
        (:NewEnumerator1
          (LocalVariables|SetBulletVelocity (+ (LocalVariables|GetBulletVelocity) (.BonusValue (Utilities|Struct|BreakS_WeaponBonus _array_element_2))))))))
  (return (LocalVariables|GetBulletVelocity)))